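; CollectiblesPool manages a capped pool of BB_Collectible actors that scroll along the X axis.
; CreateCollectible spawns one at the start X with a random height and a randomized, time-influenced speed, then stores it in the pool.
; UpdateCollectible moves each by its speed per call, recycling those past the mirrored start X with new height and speed instead of destroying them.
; Its own event graph is empty, and neither function is called within it.
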(fn `CreateCollectible`
  (if (< (`self.numberofCollectibles`) (`self.maxNumberofCollectibles`))
    (bind _returnvalue (`|SpawnActorFromClass` "/Game/Blueprints/BB_Collectible.BB_Collectible_C" (`KismetMathLibrary.MakeTransform` (`KismetMathLibrary.MakeVector` (`self.collectibleStartX`) 0.0 (`KismetMathLibrary.RandomFloatInRange` 80.0 600.0))) "Undefined" "OverrideRootScale" null null))
    (bind _speed (`/Game/Blueprints/BB_Collectible.Speed` _returnvalue))
    (set `/Game/Blueprints/BB_Collectible.Speed` (`KismetMathLibrary.RandomFloatInRange` (/ (/ (`KismetSystemLibrary.GetGameTimeInSeconds`) 10.0) _speed) _speed) _returnvalue)
    (`KismetArrayLibrary.Array_Insert` (`self.thePool`) _returnvalue (`self.numberofCollectibles`))
    (`/Engine/EditorBlueprintResources/StandardMacros.IncrementInt` (`self.numberofCollectibles`))))

(fn `UpdateCollectible`
  (bind _array_element (`self.Array Element`))
  (for (_array_element_2 _array_index) (`self.thePool`)
    (set `self.Array Element` _array_element_2)
    (set `self.Array Index` _array_index)
    (if (< (.x (`SceneComponent.K2_GetComponentLocation` (`Actor.RootComponent` _array_element_2))) (* (`self.collectibleStartX`) -1.0))
      (`SceneComponent.K2_SetWorldLocation` (`Actor.RootComponent` (`self.Array Element`)) (`KismetMathLibrary.MakeVector` (`self.collectibleStartX`) 0.0 (`KismetMathLibrary.RandomFloatInRange` 30.0 600.0)) false false)
      (bind _asbb_collectible (cast `/Game/Blueprints/BB_Collectible` (`self.Array Element`)))
      (set `/Game/Blueprints/BB_Collectible.Speed` (`KismetMathLibrary.RandomFloatInRange` 14.0 17.0) _asbb_collectible)
      (else
        (bind _asbb_collectible_2 (cast `/Game/Blueprints/BB_Collectible` _array_element))
        (`SceneComponent.K2_AddWorldOffset` (`Actor.RootComponent` _array_element) (`KismetMathLibrary.MakeVector` (- 0.0 (`/Game/Blueprints/BB_Collectible.Speed` _asbb_collectible_2))) false false)))))

(fn `UserConstructionScript`)