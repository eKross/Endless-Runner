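; AvoidablesPool is an object pool of BB_Avoidable obstacles that scroll along negative X at random heights.
; CreateAvoidable spawns one at AvoidableStartX until the maximum is reached, deriving its random speed partly from game time.
; UpdateAvoidable shifts each by its speed per call, without delta time, and recycles those past the negated start X with new height and speed.
; Its own event graph is empty and calls neither function.
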(fn `CreateAvoidable`
  (if (< (`self.numberofAvoidables`) (`self.maxNumberofAvoidables`))
    (bind _returnvalue (`|SpawnActorFromClass` "/Game/Blueprints/BB_Avoidable.BB_Avoidable_C" (`KismetMathLibrary.MakeTransform` (`KismetMathLibrary.MakeVector` (`self.avoidableStartX`) 0.0 (`KismetMathLibrary.RandomFloatInRange` 80.0 600.0))) "Undefined" "OverrideRootScale" null null))
    (bind _avoidablespeed (`/Game/Blueprints/BB_Avoidable.AvoidableSpeed` _returnvalue))
    (set `/Game/Blueprints/BB_Avoidable.AvoidableSpeed` (`KismetMathLibrary.RandomFloatInRange` (/ (/ (`KismetSystemLibrary.GetGameTimeInSeconds`) 10.0) _avoidablespeed) _avoidablespeed) _returnvalue)
    (`KismetArrayLibrary.Array_Insert` (`self.theAvoidablesPool`) _returnvalue (`self.numberofAvoidables`))
    (`/Engine/EditorBlueprintResources/StandardMacros.IncrementInt` (`self.numberofAvoidables`))))

(fn `UpdateAvoidable`
  (bind _avoidable_array_element (`self.Avoidable Array Element`))
  (for (_array_element _array_index) (`self.theAvoidablesPool`)
    (set `self.Avoidable Array Element` _array_element)
    (set `self.Array Index` _array_index)
    (if (< (.x (`SceneComponent.K2_GetComponentLocation` (`Actor.RootComponent` _array_element))) (* (`self.avoidableStartX`) -1.0))
      (`SceneComponent.K2_SetWorldLocation` (`Actor.RootComponent` (`self.Avoidable Array Element`)) (`KismetMathLibrary.MakeVector` (`self.avoidableStartX`) 0.0 (`KismetMathLibrary.RandomFloatInRange` 30.0 600.0)) false false)
      (bind _asbb_avoidable (cast `/Game/Blueprints/BB_Avoidable` (`self.Avoidable Array Element`)))
      (set `/Game/Blueprints/BB_Avoidable.AvoidableSpeed` (`KismetMathLibrary.RandomFloatInRange` 14.0 17.0) _asbb_avoidable)
      (else
        (bind _asbb_avoidable_2 (cast `/Game/Blueprints/BB_Avoidable` _avoidable_array_element))
        (`SceneComponent.K2_AddWorldOffset` (`Actor.RootComponent` _avoidable_array_element) (`KismetMathLibrary.MakeVector` (- 0.0 (`/Game/Blueprints/BB_Avoidable.AvoidableSpeed` _asbb_avoidable_2))) false false)))))

(fn `UserConstructionScript`)